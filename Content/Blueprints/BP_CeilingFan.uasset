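; Ceiling fan actor that spins its Rotor component continuously.
; On BeginPlay it caches the rotor's world rotation in Rot.
; Each Tick adds RotatorSpeed to the cached yaw, applies it as the rotor's world rotation and stores the result.
; The step is not scaled by delta time, so spin speed depends on frame rate.
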(event EventTick
  (params (DeltaSeconds :type Float%20%28single-precision%29))
  (Transformation|SetWorldRotation (Variables|Default|GetRotor) (Math|Rotator|MakeRotator (.roll (Variables|Default|GetRot)) (.pitch (Variables|Default|GetRot)) (+ (.yaw (Variables|Default|GetRot)) (Variables|Default|GetRotatorSpeed))) false false)
  (Variables|Default|SetRot (Math|Rotator|MakeRotator (.roll (Variables|Default|GetRot)) (.pitch (Variables|Default|GetRot)) (+ (.yaw (Variables|Default|GetRot)) (Variables|Default|GetRotatorSpeed)))))

(event EventBeginPlay
  (Variables|Default|SetRot (Transformation|GetWorldRotation (Variables|Default|GetRotor))))

(fn ConstructionScript)