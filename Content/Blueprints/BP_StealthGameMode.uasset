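; Stealth game mode that manages per-map objectives and their on-screen checklist, and saves the furthest completed level to the config save.
; BeginPlay randomises objective actors on Map2 by retagging them, counts "Item" actors as intel and passes itself to the StealthCharacter.
; UpdateObjectiveDisplay switches on objective type and map to update texts and checkboxes.
; SetConfig applies saved volume and material quality, but its call is disconnected.
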(event EventBeginPlay
  ;[1 1 1] Randomise level 2 objectives
  (bind _returnvalue (Game|GetCurrentLevelName true))
  (if (Utilities|Enum|Equal(Enum) _returnvalue "Map2")
    (CallFunction|RandomiseObjectives))
  ;[1 1 1] Set the number of objective items present to collect
  (bind _outactors (Actor|GetAllActorswithTag "Item"))
  (bind _output_get (Variables|Default|SetallIntel _outactors))
  (Variables|Default|SetintelMax (Utilities|Array|Length _output_get))
  ;[1 1 1] Set references in the stealth character
  (bind _outactors_2 (Actor|GetAllActorsOfClass "/Game/Blueprints/StealthCharacter.StealthCharacter_C"))
  (bind _output_get_2 (Variables|Default|SetplayerCharacter (Utilities|Array|Get(acopy) _outactors_2)))
  (Variables|/Game/Blueprints/StealthCharacter.StealthCharacter_C|Setgamemode _output_get_2 self))

(event EventTick
  (params (DeltaSeconds :type Float%20%28single-precision%29)))

(fn ConstructionScript)

(fn UpdateObjectiveDisplay
  (params (objectiveType :type EnumObjectives%20Enum :default "NewEnumerator5"))
  (bind _objectivechecks (Variables|Default|GetObjectiveChecks))
  (bind _objectivechecks_2 (Variables|Default|GetObjectiveChecks))
  ;[1 1 1] Update objectives
  (switch Utilities|FlowControl|Switch|SwitchonEnumObjectives objectiveType
    (:NewEnumerator5
      ;[1 1 1] Set objectives based on the map
      (bind _returnvalue (Game|GetCurrentLevelName true))
      (switch string _returnvalue
        (:Map1
          (CallFunction|SetMap1Objectives))
        (:Map2
          (CallFunction|SetMap2Objectives))
        (:Map3
          (CallFunction|SetMap3Objectives))))
    (:NewEnumerator0
      ;[1 1 1] Check that a key objective has been completed and update the display
      (bind _returnvalue_2 (Game|GetCurrentLevelName true))
      (switch string _returnvalue_2
        (:Map1
          (Class|CheckBox|SetIsChecked (Utilities|Array|Get(acopy) _objectivechecks_2) true))
        (:Map2
          (Class|CheckBox|SetIsChecked (Utilities|Array|Get(acopy) _objectivechecks_2 1) true))))
    (:NewEnumerator1
      ;[1 1 1] Increment the amount of objective items collected and update the display
      (bind _result (Math|Integer|IncrementInt (Variables|Default|GetintelCollected))
        (:%20%20
          (bind _output_get (Variables|Default|SetintelCollected _result))
          (Rendering|Components|TextRender|SetText (Utilities|Array|Get(acopy) (Variables|Default|GetobjectiveTexts)) (Utilities|Text|ToText(String) (Utilities|String|Append "Servers hacked for intel: " (Utilities|String|ToString(Integer) _output_get) "/" (Utilities|String|ToString(Integer) (Variables|Default|GetintelMax)))))
          (if (== (Variables|Default|GetintelCollected) (Variables|Default|GetintelMax))
            (Class|CheckBox|SetIsChecked (Utilities|Array|Get(acopy) (Variables|Default|GetObjectiveChecks)) true)))))
    (:NewEnumerator2
      ;[1 1 1] Check that an exit objective has been completed and update the display
      (Utilities|FlowControl|Sequence
        (:then_0
          (bind _returnvalue_3 (Game|GetCurrentLevelName true))
          (switch string _returnvalue_3
            (:Map1
              (Class|CheckBox|SetIsChecked (Utilities|Array|Get(acopy) _objectivechecks 1) true))
            (:Map2
              (Class|CheckBox|SetIsChecked (Utilities|Array|Get(acopy) _objectivechecks 2) false))
            (:Map3
              (Class|CheckBox|SetIsChecked (Utilities|Array|Get(acopy) _objectivechecks) false))))
        (:then_1
          ;[1 1 1] Set the furthest completed level (to determine which splash to use)
          (bind _returnvalue_4 (SaveGame|LoadGamefromSlot "config"))
          (bind _asbp_save_game (Utilities|Casting|CastToBP_SaveGame _returnvalue_4))
          (switch string _returnvalue_3
            (:Map1
              (Variables|/Game/Blueprints/BP_SaveGame.BP_SaveGame_C|SetfurthestCompletedLevel _asbp_save_game (Math|Integer|Max(Integer) (Variables|/Game/Blueprints/BP_SaveGame.BP_SaveGame_C|GetfurthestCompletedLevel _asbp_save_game) 1)))
            (:Map2
              (Variables|/Game/Blueprints/BP_SaveGame.BP_SaveGame_C|SetfurthestCompletedLevel _asbp_save_game (Math|Integer|Max(Integer) (Variables|/Game/Blueprints/BP_SaveGame.BP_SaveGame_C|GetfurthestCompletedLevel _asbp_save_game) 2)))
            (:Map3
              (Variables|/Game/Blueprints/BP_SaveGame.BP_SaveGame_C|SetfurthestCompletedLevel _asbp_save_game (Math|Integer|Max(Integer) (Variables|/Game/Blueprints/BP_SaveGame.BP_SaveGame_C|GetfurthestCompletedLevel _asbp_save_game) 3))))
          (SaveGame|SaveGametoSlot _asbp_save_game "config"))))))

(fn SetMap1Objectives
  (bind _objectivetexts (Variables|Default|GetobjectiveTexts))
  ;[1 1 1] Make third objective invisible
  (Widget|SetVisibility (Utilities|Array|Get(acopy) (Variables|Default|GetObjectiveChecks) 2) "Collapsed")
  ;[1 1 1] Set objectives
  (Rendering|Components|TextRender|SetText (Utilities|Array|Get(acopy) _objectivetexts) "Collect elevator keycard")
  (Rendering|Components|TextRender|SetText (Utilities|Array|Get(acopy) _objectivetexts 1) "Reach elevator"))

(fn SetMap2Objectives
  (bind _objectivetexts (Variables|Default|GetobjectiveTexts))
  ;[1 1 1] Set objectives
  (Rendering|Components|TextRender|SetText (Utilities|Array|Get(acopy) _objectivetexts) (Utilities|Text|ToText(String) (Utilities|String|Append "Servers hacked for intel: " (Utilities|String|ToString(Integer) (Variables|Default|GetintelCollected)) "/" (Utilities|String|ToString(Integer) (Variables|Default|GetintelMax)))))
  (Rendering|Components|TextRender|SetText (Utilities|Array|Get(acopy) _objectivetexts 1) "Hack security computer to lift elevator lockdown")
  (Rendering|Components|TextRender|SetText (Utilities|Array|Get(acopy) _objectivetexts 2) "Return to elevator"))

(fn SetMap3Objectives
  (bind _objectivechecks (Variables|Default|GetObjectiveChecks))
  ;[1 1 1] Make third objective invisible
  (Widget|SetVisibility (Utilities|Array|Get(acopy) _objectivechecks 1) "Collapsed")
  (Widget|SetVisibility (Utilities|Array|Get(acopy) _objectivechecks 2) "Collapsed")
  ;[1 1 1] Set objectives
  (Rendering|Components|TextRender|SetText (Utilities|Array|Get(acopy) (Variables|Default|GetobjectiveTexts)) "Escape the tower"))

(fn RandomiseObjectives
  (for _array_element (LocalVariables|GetallObjectiveTags)
    ;[1 1 1] Select a random objective object and set its tag
    (bind _outactors (Actor|GetAllActorswithTag _array_element))
    (bind _output_get (Variables|Default|SetaffectedObject (Utilities|Array|Get(acopy) _outactors (Math|Random|RandomInteger (Utilities|Array|Length _outactors)))))
    (Variables|/Script/Engine.Actor|SetTags _output_get (LocalVariables|GetobjectiveTag))
    (bind _asbp_objective (Utilities|Casting|CastToBP_Objective _output_get))
    ;[1 1 1] Set unique objective item parameters
    (if (Utilities|Name|Equal(Name) (Utilities|Array|Get(acopy) (Variables|/Script/Engine.Actor|GetTags _asbp_objective)) "Item")
      (Rendering|Material|SetScalarParameterValueonMaterials (Variables|/Game/Blueprints/BP_Objective.BP_Objective_C|GetCube _asbp_objective) "Offset" 0.75)
      (Rendering|Material|SetScalarParameterValueonMaterials (Variables|/Game/Blueprints/BP_Objective.BP_Objective_C|GetCube _asbp_objective) "Magnitude" 62.5)
      (else
        (Rendering|Material|SetScalarParameterValueonMaterials (Variables|/Game/Blueprints/BP_Objective.BP_Objective_C|GetCube _asbp_objective) "Glitch" 1.0)))
    ;[1 1 1] Cop out method
    (if (Utilities|Name|Equal(Name) _array_element "ServerC")
      (LocalVariables|SetobjectiveTag (Utilities|Array|MakeArray "Key")))))

(fn SetConfig
  ;[1 1 1] Create a default config save if there isn't already one
  (bind _returnvalue (SaveGame|DoesSaveGameExist "config"))
  (if _returnvalue
    _
    (else
      (bind _returnvalue_2 (SaveGame|CreateSaveGameObject "/Game/Blueprints/BP_SaveGame.BP_SaveGame_C"))
      (SaveGame|SaveGametoSlot _returnvalue_2 "config")))
  ;[1 1 1] Initialise sound classes and mixes
  (bind _returnvalue_3 (SaveGame|LoadGamefromSlot "config"))
  (bind _asbp_save_game (Utilities|Casting|CastToBP_SaveGame _returnvalue_3))
  (Audio|SetSoundMixClassOverride "/Game/Audio/SM_BGMA.SM_BGMA" "/Game/Audio/SC_BGM.SC_BGM" (Variables|/Game/Blueprints/BP_SaveGame.BP_SaveGame_C|GetsoundBGM _asbp_save_game) 1.0 1.0 true)
  (Audio|PushSoundMixModifier "/Game/Audio/SM_BGMA.SM_BGMA")
  (Audio|SetSoundMixClassOverride "/Game/Audio/SM_SFXA.SM_SFXA" "/Game/Audio/SC_SFX.SC_SFX" (Variables|/Game/Blueprints/BP_SaveGame.BP_SaveGame_C|GetsoundSFX _asbp_save_game) 1.0 1.0 true)
  (Audio|PushSoundMixModifier "/Game/Audio/SM_SFXA.SM_SFXA")
  ;[1 1 1] Set material quality
  (if (Variables|/Game/Blueprints/BP_SaveGame.BP_SaveGame_C|GetisHighQuality _asbp_save_game)
    (Development|ExecuteConsoleCommand "r.MaterialQualityLevel 1" 0)
    (else
      (Development|ExecuteConsoleCommand "r.MaterialQualityLevel 0" 0))))