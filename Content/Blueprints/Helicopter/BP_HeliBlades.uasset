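; Helicopter blade actor that spins around its yaw axis once another actor overlaps it.
; Any begin overlap stores the actor and starts the spin, while only the StealthCharacter ending its overlap stops it.
; While spinning, Tick adds a fixed step to SpinSpeed and applies it as absolute yaw, so it acts as an angle and the rotation rate depends on frame rate.
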(event EventBeginPlay)

(event EventTick
  (params (DeltaSeconds :type Float%20%28single-precision%29))
  (if (Variables|Default|GetbeginSpin)
    (bind _output_get (Variables|Default|SetspinSpeed (+ (Variables|Default|GetspinSpeed) 2.0)))
    (Transformation|SetActorRotation (Math|Rotator|MakeRotator 0.0 0.0 _output_get))))

(event Collision|EventActorBeginOverlap
  (params (OtherActor :type Actor%20Object%20Reference))
  (Variables|Default|SetPlayerRef OtherActor)
  (Variables|Default|SetbeginSpin true))

(event Collision|EventActorEndOverlap
  (params (OtherActor :type Actor%20Object%20Reference))
  (if (== OtherActor "/Game/Blueprints/StealthCharacter.StealthCharacter")
    (Variables|Default|SetbeginSpin false)))

(fn ConstructionScript)