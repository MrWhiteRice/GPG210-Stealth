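; BP_StealthMenu is an actor Blueprint that applies the saved audio and graphics settings on BeginPlay.
; SetConfig creates a default BP_SaveGame in the "config" slot if none exists, then loads it.
; The saved BGM and SFX volumes become sound mix class overrides with their mixes pushed, and the high-quality flag sets r.MaterialQualityLevel through a console command.
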(event EventBeginPlay
  (CallFunction|SetConfig))

(event EventTick
  (params (DeltaSeconds :type Float%20%28single-precision%29)))

(fn ConstructionScript)

(fn SetConfig
  ;[1 1 1] Create a default config save if there isn't already one
  (bind _returnvalue (SaveGame|DoesSaveGameExist "config"))
  (if _returnvalue
    _
    (else
      (bind _returnvalue_2 (SaveGame|CreateSaveGameObject "/Game/Blueprints/BP_SaveGame.BP_SaveGame_C"))
      (SaveGame|SaveGametoSlot _returnvalue_2 "config")))
  ;[1 1 1] Initialise sound classes and mixes
  (bind _returnvalue_3 (SaveGame|LoadGamefromSlot "config"))
  (bind _asbp_save_game (Utilities|Casting|CastToBP_SaveGame _returnvalue_3))
  (Audio|SetSoundMixClassOverride "/Game/Audio/SM_BGM.SM_BGM" "/Game/Audio/SC_BGM.SC_BGM" (Variables|/Game/Blueprints/BP_SaveGame.BP_SaveGame_C|GetsoundBGM _asbp_save_game) 1.0 1.0 true)
  (Audio|PushSoundMixModifier "/Game/Audio/SM_BGM.SM_BGM")
  (Audio|SetSoundMixClassOverride "/Game/Audio/SM_SFX.SM_SFX" "/Game/Audio/SC_SFX.SC_SFX" (Variables|/Game/Blueprints/BP_SaveGame.BP_SaveGame_C|GetsoundSFX _asbp_save_game) 1.0 1.0 true)
  (Audio|PushSoundMixModifier "/Game/Audio/SM_SFX.SM_SFX")
  ;[1 1 1] Set material quality
  (if (Variables|/Game/Blueprints/BP_SaveGame.BP_SaveGame_C|GetisHighQuality _asbp_save_game)
    (Development|ExecuteConsoleCommand "r.MaterialQualityLevel 1" 0)
    (else
      (Development|ExecuteConsoleCommand "r.MaterialQualityLevel 0" 0))))