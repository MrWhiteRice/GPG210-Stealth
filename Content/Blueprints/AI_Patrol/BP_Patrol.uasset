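; BP_Patrol is a stealth-game patrol AI that seeds its Blackboard with patrol points and a start index.
; Each tick, AI sight perception checks for the StealthCharacter and updates canSee.
; When seen, the player's light level drives aggroPercent: Light maxes it, Shaded raises it, Dark lowers it.
; When unseen it decays, with a one-second Delay and boolean gates throttling updates and delaying loss of sight.
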(event EventBeginPlay
  (bind _self self)
  (bind _returnvalue (AI|GetBlackboard _self))
  (bind _outactors (Actor|GetAllActorsOfClass "/Game/Blueprints/StealthCharacter.StealthCharacter_C"))
  (Variables|Default|SetPlayerRef (Utilities|Array|Get(acopy) _outactors))
  (AI|Components|Blackboard|SetValueasObject _returnvalue (Utilities|Name|MakeLiteralName "Points") (Variables|Default|GetPatrolPoints))
  (Class|BlackboardComponent|SetValueasInt _returnvalue (Utilities|Name|MakeLiteralName "CurrentPatrolPoint") (Variables|Default|GetStartPoint)))

(event EventTick
  (params (DeltaSeconds :type Float%20%28single-precision%29))
  (bind _returnvalue (Utilities|Name|MakeLiteralName "canSee"))
  (bind _returnvalue_2 (Utilities|Name|MakeLiteralName "aggroPercent"))
  (bind _returnvalue_3 (Utilities|Name|MakeLiteralName "aggroPercent"))
  (bind _returnvalue_4 (Utilities|Name|MakeLiteralName "aggroPercent"))
  (bind _self self)
  (bind _self_2 self)
  (bind _returnvalue_5 (AI|GetBlackboard _self))
  (bind _returnvalue_6 (AI|GetBlackboard _self_2))
  (bind _returnvalue_7 (Class|BlackboardComponent|GetValueasFloat _returnvalue_6 _returnvalue_2))
  (bind _returnvalue_8 (Class|BlackboardComponent|GetValueasFloat _returnvalue_6 _returnvalue_3))
  (bind _returnvalue_9 (- _returnvalue_8 5.0))
  (bind _returnvalue_10 (+ _returnvalue_7 5.0))
  (for _array_element (Class|AIPerceptionComponent|GetPerceivedActors (Variables|Default|GetAIPerception) "/Script/AIModule.AISense_Sight")
    (if (== _array_element (Variables|Default|GetPlayerRef))
      (Variables|Default|Setyeetcheck false)
      (AI|Components|Blackboard|SetValueasBool _returnvalue_5 _returnvalue true)
      (if (ScalableFloat|GetValueasBool (AI|GetBlackboard self) (Utilities|Name|MakeLiteralName "canSee"))
        (bind _outactors (Actor|GetAllActorsOfClass "/Game/Blueprints/StealthCharacter.StealthCharacter_C"))
        (if (Variables|Default|Gettick)
          (Variables|Default|Settick false)
          (switch Utilities|FlowControl|Switch|SwitchonEnumLight (Variables|/Game/Blueprints/StealthCharacter.StealthCharacter_C|GetplayerLightLevel (Utilities|Array|Get(acopy) _outactors))
            (:NewEnumerator0
              (AI|Components|Blackboard|SetValueasFloat _returnvalue_6 _returnvalue_4 1e+02 :!label _label))
            (:NewEnumerator1
              (if (>= _returnvalue_10 1e+02)
                (goto _label)
                (else
                  (AI|Components|Blackboard|SetValueasFloat _returnvalue_6 _returnvalue_4 _returnvalue_10))))
            (:NewEnumerator2
              (if (<= _returnvalue_9 0.0) :!label _label_2
                (AI|Components|Blackboard|SetValueasFloat _returnvalue_6 _returnvalue_4 0.0)
                (else
                  (AI|Components|Blackboard|SetValueasFloat _returnvalue_6 _returnvalue_4 _returnvalue_9)))))
          (Utilities|FlowControl|Delay 1.0)
          (Variables|Default|Settick true)
          (Variables|Default|Setyeetcheck true))
        (elif (Variables|Default|Gettick)
          (Variables|Default|Settick false)
          (goto _label_2)))))
  (if (Variables|Default|Getyeetcheck)
    (AI|Components|Blackboard|SetValueasBool _returnvalue_5 _returnvalue false)
    (if (ScalableFloat|GetValueasBool (AI|GetBlackboard self) (Utilities|Name|MakeLiteralName "canSee"))
      (bind _outactors_2 (Actor|GetAllActorsOfClass "/Game/Blueprints/StealthCharacter.StealthCharacter_C"))
      (if (Variables|Default|Gettick)
        (Variables|Default|Settick false)
        (switch Utilities|FlowControl|Switch|SwitchonEnumLight (Variables|/Game/Blueprints/StealthCharacter.StealthCharacter_C|GetplayerLightLevel (Utilities|Array|Get(acopy) _outactors_2))
          (:NewEnumerator0
            (AI|Components|Blackboard|SetValueasFloat _returnvalue_6 _returnvalue_4 1e+02 :!label _label_3))
          (:NewEnumerator1
            (if (>= _returnvalue_10 1e+02)
              (goto _label_3)
              (else
                (AI|Components|Blackboard|SetValueasFloat _returnvalue_6 _returnvalue_4 _returnvalue_10))))
          (:NewEnumerator2
            (if (<= _returnvalue_9 0.0) :!label _label_4
              (AI|Components|Blackboard|SetValueasFloat _returnvalue_6 _returnvalue_4 0.0)
              (else
                (AI|Components|Blackboard|SetValueasFloat _returnvalue_6 _returnvalue_4 _returnvalue_9)))))
        (Utilities|FlowControl|Delay 1.0)
        (Variables|Default|Settick true)
        (Variables|Default|Setyeetcheck true))
      (elif (Variables|Default|Gettick)
        (Variables|Default|Settick false)
        (goto _label_4)))))

(fn ConstructionScript)