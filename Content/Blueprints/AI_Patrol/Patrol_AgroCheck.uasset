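; Behavior tree tick node for patrol AI that checks whether aggro is high enough to start following the player.
; Each tick it uses a cached AIC_Patrol controller to read the blackboard's aggroPercent, and at the threshold sets followTarget to the first StealthCharacter found.
; Disconnected graphs hold unused logic for raising or decaying aggro from sight and player light level, plus a debug line trace.
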(event EventTick
  (params (OwnerActor :type Actor%20Object%20Reference) (DeltaSeconds :type Float%20%28single-precision%29))
  (if (!= (Variables|Default|GetAI_CON_Ref) 0)
    _
    (else
      (bind _asaic_patrol (Utilities|Casting|CastToAIC_Patrol OwnerActor))
      (Variables|Default|SetAI_CON_Ref _asaic_patrol)))
  (if (>= (Class|BlackboardComponent|GetValueasFloat (AI|GetBlackboard (Variables|Default|GetAI_CON_Ref)) (Utilities|Name|MakeLiteralName "aggroPercent")) 1e+02)
    (bind _outactors (Actor|GetAllActorsOfClass "/Game/Blueprints/StealthCharacter.StealthCharacter_C"))
    (AI|Components|Blackboard|SetValueasObject (AI|GetBlackboard (Variables|Default|GetAI_CON_Ref)) (Utilities|Name|MakeLiteralName "followTarget") (Utilities|Array|Get(acopy) _outactors))))