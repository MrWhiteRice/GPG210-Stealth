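; Behavior tree task for patrol AI that starts moving the controlled pawn toward the blackboard's follow target.
; It caches the AIC_Patrol controller and, right after issuing AIMoveTo, finishes successfully if canSee is set.
; Otherwise, below full aggroPercent it prints a debug string, sets searching, clears followTarget and finishes.
; With the target unseen at full aggro, the task never calls FinishExecute.
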(event EventReceiveExecute
  (params (OwnerActor :type Actor%20Object%20Reference))
  (if (!= (Variables|Default|GetAI_CON_Ref) 0)
    _
    (else
      (bind _asaic_patrol (Utilities|Casting|CastToAIC_Patrol OwnerActor))
      (Variables|Default|SetAI_CON_Ref _asaic_patrol)))
  (AI|AIMoveTo (Pawn|GetControlledPawn (Variables|Default|GetAI_CON_Ref)) "0, 0, 0" (AI|BehaviorTree|GetBlackboardValueasActor (Variables|Default|GetTargetToFollow)) 5e+01 false
    (:then
      (if (ScalableFloat|GetValueasBool (AI|GetBlackboard (Variables|Default|GetAI_CON_Ref)) (Utilities|Name|MakeLiteralName "canSee"))
        (AI|BehaviorTree|FinishExecute true :!label _label)
        (elif (< (Class|BlackboardComponent|GetValueasFloat (AI|GetBlackboard (Variables|Default|GetAI_CON_Ref)) (Utilities|Name|MakeLiteralName "aggroPercent")) 1e+02)
          (Development|PrintString "Hello")
          (AI|Components|Blackboard|SetValueasBool (AI|GetBlackboard (Variables|Default|GetAI_CON_Ref)) (Utilities|Name|MakeLiteralName "searching") true)
          (AI|Components|Blackboard|SetValueasObject (AI|GetBlackboard (Variables|Default|GetAI_CON_Ref)) (Utilities|Name|MakeLiteralName "followTarget") 0)
          (goto _label))))))