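; Behavior tree task for patrol AI attacks that gives the player a slow-motion dodge window.
; On execute it caches the controller and player; within close range and off cooldown, it starts the dodge, records the attacker and slows global time.
; It finishes as failed, except when in range during cooldown, where it never finishes.
; A hitbox overlap handler repeats the dodge without an attacker; level-reload nodes are disconnected.
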(event OnComponentBeginOverlap(CombatHitboxCapsule)
  (params (OverlappedComponent :type Primitive%20Component%20Object%20Reference) (OtherActor :type Actor%20Object%20Reference) (OtherComp :type Primitive%20Component%20Object%20Reference) (OtherBodyIndex :type Integer) (bFromSweep :type Boolean) (SweepResult :type Hit%20Result%20Structure%20%28by%20ref%29))
  ;[1 1 1] Tell player character to try to dodge
  (bind _asstealth_character (Utilities|Casting|CastToStealthCharacter OtherActor))
  (if (<= (Variables|/Game/Blueprints/StealthCharacter.StealthCharacter_C|GetdodgeCooldown _asstealth_character) 0.0)
    (Variables|/Game/Blueprints/StealthCharacter.StealthCharacter_C|SetdodgeCooldown _asstealth_character 2e+01)
    (Variables|/Game/Blueprints/StealthCharacter.StealthCharacter_C|SetisDodging _asstealth_character true)
    (Variables|/Game/Blueprints/StealthCharacter.StealthCharacter_C|SetdodgeEnd _asstealth_character (+ (Utilities|Time|GetGameTimeinSeconds) (/ (Variables|/Game/Blueprints/StealthCharacter.StealthCharacter_C|GetdodgeDuration _asstealth_character) 4.0)))
    (Variables|/Game/Blueprints/StealthCharacter.StealthCharacter_C|SetattackingEnemy _asstealth_character 0)
    (Utilities|Time|SetGlobalTimeDilation 0.25)
    (else
      (Development|PrintString "dodge expired"))))

(event EventReceiveExecute
  (params (OwnerActor :type Actor%20Object%20Reference)))

(event EventReceiveExecuteAI
  (params (OwnerController :type AI%20Controller%20Object%20Reference) (ControlledPawn :type Pawn%20Object%20Reference))
  (if (!= (Variables|Default|GetAI_CON_Ref) 0)
    _
    (else
      (bind _asaic_patrol (Utilities|Casting|CastToAIC_Patrol OwnerController))
      (Variables|Default|SetAI_CON_Ref _asaic_patrol)))
  (if (!= (Variables|Default|GetplayerRef) 0)
    _
    (else
      (bind _outactors (Actor|GetAllActorsOfClass "/Game/Blueprints/StealthCharacter.StealthCharacter_C"))
      (Variables|Default|SetplayerRef (Utilities|Array|Get(acopy) _outactors))))
  (if (< (Math|Vector|VectorLength (- (Transformation|GetActorLocation ControlledPawn) (Transformation|GetActorLocation (Variables|Default|GetplayerRef)))) 1e+02)
    (if (<= (Variables|/Game/Blueprints/StealthCharacter.StealthCharacter_C|GetdodgeCooldown (Variables|Default|GetplayerRef)) 0.0)
      (Variables|/Game/Blueprints/StealthCharacter.StealthCharacter_C|SetdodgeCooldown (Variables|Default|GetplayerRef) 2e+01)
      (Variables|/Game/Blueprints/StealthCharacter.StealthCharacter_C|SetisDodging (Variables|Default|GetplayerRef) true)
      (Development|PrintString "Hello")
      (Variables|/Game/Blueprints/StealthCharacter.StealthCharacter_C|SetdodgeEnd (Variables|Default|GetplayerRef) (+ (Utilities|Time|GetGameTimeinSeconds) (/ (Variables|/Game/Blueprints/StealthCharacter.StealthCharacter_C|GetdodgeDuration (Variables|Default|GetplayerRef)) 4.0)))
      (Variables|/Game/Blueprints/StealthCharacter.StealthCharacter_C|SetattackingEnemy (Variables|Default|GetplayerRef) (Variables|Default|GetAI_CON_Ref))
      (Utilities|Time|SetGlobalTimeDilation 0.25)
      (AI|BehaviorTree|FinishExecute false :!label _label))
    (else
      (goto _label))))