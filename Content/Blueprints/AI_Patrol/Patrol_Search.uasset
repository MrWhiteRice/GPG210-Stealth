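; Behavior tree task for AI patrol that sends the controlled pawn to a search point.
; When the blackboard flag isSearching is true, it issues an AI MoveTo toward the NextPoint vector, using the pawn from the AIREFERENCE controller.
; It clears isSearching on the move node's immediate output rather than on arrival.
; The graph never calls Finish Execute.
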(event EventReceiveExecute
  (params (OwnerActor :type Actor%20Object%20Reference))
  (bind _returnvalue (AI|GetBlackboard OwnerActor))
  (if (ScalableFloat|GetValueasBool _returnvalue (Utilities|Name|MakeLiteralName "isSearching"))
    (AI|AIMoveTo (Pawn|GetControlledPawn (Variables|Default|GetAI%20REFERENCE)) (AI|Components|Blackboard|GetValueasVector _returnvalue (Utilities|Name|MakeLiteralName "NextPoint")) 0 5.0 false
      (:then
        (AI|Components|Blackboard|SetValueasBool _returnvalue (Utilities|Name|MakeLiteralName "isSearching") false)))))