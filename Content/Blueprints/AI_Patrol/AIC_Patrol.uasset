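; AIC_Patrol is an AI controller that drives patrolling pawns through the BT_Patrol behavior tree and BB_Patrol blackboard.
; On BeginPlay it assigns the blackboard and starts the tree, leaving the patrol logic to those assets.
; Disconnected leftover nodes would set the HomeLocation key from the pawn's position or a random PP1-tagged actor, but they never run.
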(event EventTick
  (params (DeltaSeconds :type Float%20%28single-precision%29)))

(event EventBeginPlay
  (Class|AIController|UseBlackboard "/Game/Blueprints/AI_Patrol/BB_Patrol.BB_Patrol")
  (AI|RunBehaviorTree "/Game/Blueprints/AI_Patrol/BT_Patrol.BT_Patrol"))

(fn ConstructionScript)