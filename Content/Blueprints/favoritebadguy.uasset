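; Enemy AI pawn for a stealth game that patrols between two points and chases the player once spotted.
; Patrol loops through AIMoveTo calls, recursing after the second point.
; PawnSensing latches CanSee when it sees a StealthCharacter outside shadow, and Tick then reissues a move toward that character; nothing here clears the flag.
; Tick also yaws EnemyIndicator to face the player's follow camera.
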(event OnSeePawn(PawnSensing)
  (params (Pawn :type Pawn%20Object%20Reference))
  ;[1 1 1] Comment
  (bind _asstealth_character (Utilities|Casting|CastToStealthCharacter Pawn))
  (if (not (Variables|/Game/Blueprints/StealthCharacter.StealthCharacter_C|GetisInShadow _asstealth_character))
    (Variables|Default|SetCanSee true)))

(event Custom|FUNCTION%20PATROL
  ;[1 1 1] Patrol
  (AI|AIMoveTo self "0, 0, 0" (Variables|Default|GetPatrolPoint1) 5.0 false
    (:OnSuccess
      (AI|AIMoveTo self "0, 0, 0" (Variables|Default|GetPatrolPoint2) 5.0 false
        (:OnSuccess
          (CallFunction|FUNCTIONPATROL))))))

(event EventBeginPlay
  ;[1 1 1] Start patrol
  (CallFunction|FUNCTIONPATROL)
  ;[1 1 1] Get player character
  (bind _outactors (Actor|GetAllActorsOfClass "/Game/Blueprints/StealthCharacter.StealthCharacter_C"))
  (Variables|Default|SetplayerCamera (Variables|/Game/Blueprints/StealthCharacter.StealthCharacter_C|GetFollowCamera (Utilities|Array|Get(acopy) _outactors))))

(event EventTick
  (params (DeltaSeconds :type Float%20%28single-precision%29))
  (bind _enemyindicator (Variables|Default|GetenemyIndicator))
  (Utilities|FlowControl|Sequence
    (:then_0
      ;[1 1 1] Rotate indicator to face player camera
      (Transformation|SetWorldRotation _enemyindicator (Math|Rotator|MakeRotator 0.0 0.0 (.yaw (Math|Rotator|FindLookatRotation (Transformation|GetWorldLocation _enemyindicator) (Transformation|GetWorldLocation (Variables|Default|GetplayerCamera))))) false false))
    (:then_1
      ;[1 1 1] On update, turn off seen
      (if (Variables|Default|GetCanSee)
        (AI|AIMoveTo self "0, 0, 0" (stale OnSeePawn(PawnSensing) _asstealth_character) 5.0 false)))))

(fn ConstructionScript)