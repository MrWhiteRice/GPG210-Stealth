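; BP_KeyCard is a key card actor that spins and bobs in place, with no pickup logic in its graphs.
; BeginPlay caches its starting location and rotation.
; Tick adds RotationSpeed to yaw each frame, unscaled by delta time, and sets the transform.
; Height lerps around the origin using sine of lifetime as alpha; its negative half extrapolates, so the bob spans +3 to -1 times MaxBob.
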(event EventBeginPlay
  (Variables|Default|SetOrigin (Transformation|GetActorLocation))
  (Variables|Default|SetRot (Transformation|GetActorRotation)))

(event EventTick
  (params (DeltaSeconds :type Float%20%28single-precision%29))
  (bind _origin (Variables|Default|GetOrigin))
  (bind _origin_2 (Variables|Default|GetOrigin))
  (bind _maxbob (Variables|Default|GetMaxBob))
  (bind _output_get (Variables|Default|SetRot (Math|Rotator|MakeRotator (.roll (Variables|Default|GetRot)) (.pitch (Variables|Default|GetRot)) (+ (.yaw (Variables|Default|GetRot)) (Variables|Default|GetRotationSpeed)))))
  (Transformation|SetActorTransform (Math|Transform|MakeTransform (Math|Vector|Lerp(Vector) (Math|Vector|MakeVector (.x _origin_2) (.y _origin_2) (+ (.z _origin_2) _maxbob)) (Math|Vector|MakeVector (.x _origin) (.y _origin) (- (.z _origin) _maxbob)) (Math|Trig|Sin(Radians) (Actor|GetGameTimeSinceCreation))) _output_get "1,1,1")))

(fn ConstructionScript)