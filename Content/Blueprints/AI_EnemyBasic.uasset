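; Basic AI enemy that detects pawns by sight and passes player information to its Blackboard.
; On seeing any pawn, PawnSensing applies BB_EnemyBasic and sets Aggro, then stores the pawn as Player only if it is a StealthCharacter.
; Every Tick, it looks up all StealthCharacters and writes the first one's location to the Point key, whether or not it has been seen.
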(event OnSeePawn(PawnSensing)
  (params (Pawn :type Pawn%20Object%20Reference))
  (bind _blackboardcomponent (Class|AIController|UseBlackboard (AI|GetAIController self) "/Game/Blueprints/BB_EnemyBasic.BB_EnemyBasic"))
  (AI|Components|Blackboard|SetValueasBool _blackboardcomponent (Utilities|Name|MakeLiteralName "Aggro") true)
  (bind _asstealth_character (Utilities|Casting|CastToStealthCharacter Pawn))
  (bind _output_get (Variables|Default|SetPlayer _asstealth_character))
  (AI|Components|Blackboard|SetValueasObject _blackboardcomponent (Utilities|Name|MakeLiteralName "Player") _output_get))

(event EventTick
  (params (DeltaSeconds :type Float%20%28single-precision%29))
  (bind _outactors (Actor|GetAllActorsOfClass "/Game/Blueprints/StealthCharacter.StealthCharacter_C"))
  (AI|Components|Blackboard|SetValueasVector (AI|GetBlackboard 0) (Utilities|Name|MakeLiteralName "Point") (Transformation|GetActorLocation (Utilities|Array|Get(acopy) _outactors))))

(fn ConstructionScript)