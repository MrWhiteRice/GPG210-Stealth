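; BP_ElevatorButton is an elevator button actor that animates its Cube's material while IsOn is set; it holds no press or elevator logic.
; BeginPlay creates a dynamic material instance, and Tick drives its Trans parameter with a sine of the actor's lifetime.
; When Random is set, the sine is offset to stay positive and scaled by a fresh random factor each frame, giving a flickering pulse.
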(event EventBeginPlay
  (bind _returnvalue (Rendering|Material|CreateDynamicMaterialInstance (Variables|Default|GetCube) 0 0 "None" :!class /Script/Engine.PrimitiveComponent))
  (Variables|Default|SetMatInstance _returnvalue))

(event Collision|EventActorBeginOverlap
  (params (OtherActor :type Actor%20Object%20Reference)))

(event EventTick
  (params (DeltaSeconds :type Float%20%28single-precision%29))
  (bind _returnvalue (Actor|GetGameTimeSinceCreation))
  (bind _matinstance (Variables|Default|GetMatInstance))
  (bind _returnvalue_2 (Math|Trig|Sin(Radians) _returnvalue))
  (if (Variables|Default|GetisOn)
    (if (Variables|Default|Getrandom)
      (Rendering|Material|SetScalarParameterValue _matinstance "Trans" (* (+ _returnvalue_2 1.5) (Math|Random|RandomFloatinRange 0.5 1.0)) :!class /Script/Engine.MaterialInstanceDynamic)
      (else
        (Rendering|Material|SetScalarParameterValue _matinstance "Trans" _returnvalue_2 :!class /Script/Engine.MaterialInstanceDynamic)))))

(fn ConstructionScript)