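; Behavior tree task in the AI_Drone folder that picks a random patrol destination for the drone.
; On Tick it reads the PatrolPoints blackboard object, picks a random actor from its Points array and writes that location to movePosition.
; It then finishes as failed even after a successful write; a failed cast leaves it unfinished.
; A leftover debug string prints on each tick.
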(event EventTick
  (params (OwnerActor :type Actor%20Object%20Reference) (DeltaSeconds :type Float%20%28single-precision%29))
  (bind _returnvalue (AI|GetBlackboard OwnerActor))
  (Development|PrintString "asdasdasdasdasd")
  (bind _asbp_patrol_points (Utilities|Casting|CastToBP_PatrolPoints (AI|Components|Blackboard|GetValueasObject _returnvalue (Utilities|Name|MakeLiteralName "PatrolPoints"))))
  (AI|Components|Blackboard|SetValueasVector _returnvalue (Utilities|Name|MakeLiteralName "movePosition") (Transformation|GetActorLocation (Utilities|Array|Get(acopy) (Variables|/Game/Blueprints/AI_Generic/BP_PatrolPoints.BP_PatrolPoints_C|GetPoints _asbp_patrol_points) (Math|Random|RandomInteger (Utilities|Array|Length (Variables|/Game/Blueprints/AI_Generic/BP_PatrolPoints.BP_PatrolPoints_C|GetPoints _asbp_patrol_points))))))
  (AI|BehaviorTree|FinishExecute false))