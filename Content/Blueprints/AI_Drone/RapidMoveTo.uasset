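; Behavior tree task that sends the AI drone to the current position of the first StealthCharacter in the level.
; On execute it caches the AIC_Drone controller, writes that position to the lastKnowLoc blackboard key and starts an AI move to it.
; A recharge sound plays at the drone as the move starts.
; The task finishes only when the move succeeds, with no handling for a failed move.
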(event EventReceiveExecute
  (params (OwnerActor :type Actor%20Object%20Reference))
  (bind _outactors (Actor|GetAllActorsOfClass "/Game/Blueprints/StealthCharacter.StealthCharacter_C"))
  (if (!= (Variables|Default|GetAI_CON_Ref) 0)
    _
    (else
      (bind _asaic_drone (Utilities|Casting|CastToAIC_Drone OwnerActor))
      (Variables|Default|SetAI_CON_Ref _asaic_drone)))
  (AI|Components|Blackboard|SetValueasVector (AI|GetBlackboard OwnerActor) (Utilities|Name|MakeLiteralName "lastKnowLoc") (Transformation|GetActorLocation (Utilities|Array|Get(acopy) _outactors)))
  (AI|AIMoveTo (Pawn|GetControlledPawn (Variables|Default|GetAI_CON_Ref)) (Transformation|GetActorLocation (Utilities|Array|Get(acopy) _outactors)) 0 5e+01 false
    (:then
      (Audio|PlaySoundatLocation "/Game/Audio/AC_TeleRecharge.AC_TeleRecharge" (Transformation|GetActorLocation (Pawn|GetControlledPawn (Variables|Default|GetAI_CON_Ref))) "0, 0, 0" 1.0 1.0 0.0 0 0 0))
    (:OnSuccess
      (AI|BehaviorTree|FinishExecute true))))