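; BP_TempDrone is a temporary AI drone that patrols and watches for the player's StealthCharacter through sight perception.
; BeginPlay writes its Pat object to the blackboard's PatrolPoints key and caches the first StealthCharacter found as the player.
; Each Tick loops over sight-perceived actors, setting the "viewing" key by whether each is the player.
; The last actor decides the value, and an empty list leaves it unchanged.
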(event EventBeginPlay
  (AI|Components|Blackboard|SetValueasObject (AI|GetBlackboard self) (Utilities|Name|MakeLiteralName "PatrolPoints") (Variables|Default|GetPat))
  (bind _outactors (Actor|GetAllActorsOfClass "/Game/Blueprints/StealthCharacter.StealthCharacter_C"))
  (Variables|Default|SetplayerRef (Utilities|Array|Get(acopy) _outactors)))

(event EventTick
  (params (DeltaSeconds :type Float%20%28single-precision%29))
  (bind _returnvalue (Utilities|Name|MakeLiteralName "viewing"))
  (bind _self self)
  (bind _returnvalue_2 (AI|GetBlackboard _self))
  (for _array_element (Class|AIPerceptionComponent|GetPerceivedActors (Variables|Default|GetAIPerception) "/Script/AIModule.AISense_Sight")
    (if (== _array_element (Variables|Default|GetplayerRef))
      (AI|Components|Blackboard|SetValueasBool _returnvalue_2 _returnvalue true)
      (else
        (AI|Components|Blackboard|SetValueasBool _returnvalue_2 _returnvalue false)))))

(fn ConstructionScript)