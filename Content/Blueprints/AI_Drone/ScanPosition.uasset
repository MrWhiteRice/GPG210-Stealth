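; Drone behavior tree task that scans for the player's stealth character and raises the alarm when it is spotted.
; Each tick, using a cached AIC_Drone, it sets isChasing from whether the character is within close range and the blackboard's viewing flag is set.
; On detection it also raises aggroPercent on every BP_Patrol's blackboard, calling FinishExecute inside that loop.
; Otherwise it clears isChasing and finishes successfully; both outcomes print debug strings.
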(event EventTick
  (params (OwnerActor :type Actor%20Object%20Reference) (DeltaSeconds :type Float%20%28single-precision%29))
  (bind _returnvalue (AI|GetBlackboard OwnerActor))
  (bind _returnvalue_2 (Utilities|Name|MakeLiteralName "isChasing"))
  (if (!= (Variables|Default|Getaic) 0)
    _
    (else
      (bind _asaic_drone (Utilities|Casting|CastToAIC_Drone (AI|GetAIController OwnerActor)))
      (bind _output_get (Variables|Default|Setaic _asaic_drone))))
  (bind _outactors (Actor|GetAllActorsOfClass "/Game/Blueprints/StealthCharacter.StealthCharacter_C"))
  (if (<= (Math|Vector|VectorLength (- (Transformation|GetActorLocation (Utilities|Array|Get(acopy) _outactors)) (Transformation|GetActorLocation (Pawn|GetControlledPawn _output_get)))) 3e+02)
    (if (ScalableFloat|GetValueasBool _returnvalue (Utilities|Name|MakeLiteralName "viewing"))
      (AI|Components|Blackboard|SetValueasBool _returnvalue _returnvalue_2 true)
      (Development|PrintString "ye")
      ;[1 1 1] Alert all patrol enemies
      (bind _outactors_2 (Actor|GetAllActorsOfClass "/Game/Blueprints/AI_Patrol/BP_Patrol.BP_Patrol_C"))
      (for _array_element _outactors_2
        (AI|Components|Blackboard|SetValueasFloat (AI|GetBlackboard (Pawn|GetController _array_element)) (Utilities|Name|MakeLiteralName "aggroPercent") 3e+02)
        (AI|BehaviorTree|FinishExecute true))
      (else
        (AI|Components|Blackboard|SetValueasBool _returnvalue _returnvalue_2 false :!label _label)
        (Development|PrintString "no")
        (AI|BehaviorTree|FinishExecute true)))
    (else
      (goto _label))))