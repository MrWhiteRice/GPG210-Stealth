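; AI controller for the AITEST enemy that sets up its blackboard and runs its behavior tree.
; On BeginPlay it loads BB_AITEST, stores its own location as the Start key and the first StealthCharacter found as the Player key.
; It then starts BT_AITEST, which takes over the AI's behavior.
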(event EventBeginPlay
  (bind _self self)
  (bind _returnvalue (AI|GetBlackboard _self))
  (Class|AIController|UseBlackboard "/Game/Blueprints/AI_1/BB_AITEST.BB_AITEST")
  (AI|Components|Blackboard|SetValueasVector _returnvalue (Utilities|Name|MakeLiteralName "Start") (Transformation|GetActorLocation))
  (bind _outactors (Actor|GetAllActorsOfClass "/Game/Blueprints/StealthCharacter.StealthCharacter_C"))
  (AI|Components|Blackboard|SetValueasObject _returnvalue (Utilities|Name|MakeLiteralName "Player") (Utilities|Array|Get(acopy) _outactors))
  (AI|RunBehaviorTree "/Game/Blueprints/AI_1/BT_AITEST.BT_AITEST"))

(fn ConstructionScript)