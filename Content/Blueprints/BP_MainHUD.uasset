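; BP_MainHUD sets up the stealth game's gameplay UI when play begins.
; It creates the BP_GameplayUI widget and adds it to the viewport.
; It passes the widget and its intel text to BP_StealthGameMode, then triggers an intel display update.
; It also gives StealthCharacter the teleport bar, finding both actors by taking the first GetAllActorsOfClass result.
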(event EventBeginPlay
  ;[1 1 1] Create the gameplay ui widget
  (bind _returnvalue (UserInterface|CreateWidget "/Game/Blueprints/BP_GameplayUI.BP_GameplayUI_C"))
  (UserInterface|Viewport|AddtoViewport _returnvalue 0)
  ;[1 1 1] Set a reference to the UI and text in the gamemode and call for it to update
  (bind _outactors (Actor|GetAllActorsOfClass "/Game/Blueprints/BP_StealthGameMode.BP_StealthGameMode_C"))
  (Variables|/Game/Blueprints/BP_StealthGameMode.BP_StealthGameMode_C|SetgameplayUI (Utilities|Array|Get(acopy) _outactors) _returnvalue)
  (Variables|/Game/Blueprints/BP_StealthGameMode.BP_StealthGameMode_C|SetintelText (Utilities|Array|Get(acopy) _outactors) (Variables|/Game/Blueprints/BP_GameplayUI.BP_GameplayUI_C|GettextIntelDisplay _returnvalue))
  (Default|UpdateIntelDisplay (Utilities|Array|Get(acopy) _outactors))
  (bind _outactors_2 (Actor|GetAllActorsOfClass "/Game/Blueprints/StealthCharacter.StealthCharacter_C"))
  (Variables|/Game/Blueprints/StealthCharacter.StealthCharacter_C|SetteleportBarObject (Utilities|Array|Get(acopy) _outactors_2) (Variables|/Game/Blueprints/BP_GameplayUI.BP_GameplayUI_C|GetteleUIBar _returnvalue)))

(event Collision|EventActorBeginOverlap
  (params (OtherActor :type Actor%20Object%20Reference)))

(event EventTick
  (params (DeltaSeconds :type Float%20%28single-precision%29)))

(fn ConstructionScript)