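; AI controller for the Nullifier enemy that seeds its blackboard and starts its behavior tree.
; On BeginPlay it uses BB_Nullifier and stores the pawn's spawn location as its home.
; It copies the follow flag, master object and patrol array object from the BP_AI_Nullifier pawn into the blackboard.
; It then runs BT_Nullifier, which receives all decision-making; Tick is empty.
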(event EventBeginPlay
  (bind _returnvalue (Pawn|GetControlledPawn))
  (bind _self self)
  (bind _returnvalue_2 (AI|GetBlackboard _self))
  (Class|AIController|UseBlackboard "/Game/Blueprints/AI_Nullifier/BB_Nullifier.BB_Nullifier")
  (AI|Components|Blackboard|SetValueasVector _returnvalue_2 (Variables|Default|GethomeLocationKey) (Transformation|GetActorLocation _returnvalue))
  (bind _asbp_ai_nullifier (Utilities|Casting|CastToBP_AI_Nullifier _returnvalue))
  (AI|Components|Blackboard|SetValueasBool _returnvalue_2 (Variables|Default|GetisFollowingKey) (Variables|/Game/Blueprints/AI_Nullifier/BP_AI_Nullifier.BP_AI_Nullifier_C|GetisFollowing _asbp_ai_nullifier))
  (AI|Components|Blackboard|SetValueasObject _returnvalue_2 (Variables|Default|GetmasterObjectKey) (Variables|/Game/Blueprints/AI_Nullifier/BP_AI_Nullifier.BP_AI_Nullifier_C|GetmasterObject _asbp_ai_nullifier))
  (AI|Components|Blackboard|SetValueasObject _returnvalue_2 (Utilities|Name|MakeLiteralName "pointArray") (Variables|/Game/Blueprints/AI_Nullifier/BP_AI_Nullifier.BP_AI_Nullifier_C|GetpatrolArrayObject _asbp_ai_nullifier))
  (AI|RunBehaviorTree "/Game/Blueprints/AI_Nullifier/BT_Nullifier.BT_Nullifier"))

(event EventTick
  (params (DeltaSeconds :type Float%20%28single-precision%29)))

(fn ConstructionScript)