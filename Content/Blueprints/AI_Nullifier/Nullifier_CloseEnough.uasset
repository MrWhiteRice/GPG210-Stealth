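; Behavior tree decorator for the Nullifier AI that gates a branch on its pawn's distance from the TargetToFollow blackboard actor.
; It casts the owner to BP_AIC_Nullifier, then compares the straight-line distance between the controlled pawn and the target against AcceptableDistance.
; Despite the CloseEnough name, the check passes when the distance is at or beyond that threshold.
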(fn PerformConditionCheck
  (params (OwnerActor :type Actor%20Object%20Reference))
  ;[1 1 1] Get a reference to the controller
  (bind _asbp_aic_nullifier (Utilities|Casting|CastToBP_AIC_Nullifier OwnerActor))
  (bind _output_get (Variables|Default|SetnullifierAIC _asbp_aic_nullifier))
  ;[1 1 1] Determine if the AI is close enough to the target
  (return (>= (Math|Vector|VectorLength (- (Transformation|GetActorLocation (AI|BehaviorTree|GetBlackboardValueasActor (Variables|Default|GettargetToFollow))) (Transformation|GetActorLocation (Pawn|GetControlledPawn _output_get)))) (Variables|Default|GetacceptableDistance))))