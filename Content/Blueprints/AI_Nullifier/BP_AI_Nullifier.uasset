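; BP_AI_Nullifier is an AI enemy that shows the player how aware it is through an overhead awareness bar widget.
; On BeginPlay it caches the StealthCharacter's follow camera, its BP_AIC_Nullifier controller and the BP_EnemyAwareness progress bar.
; Each tick it yaws the widget toward the camera and reads the blackboard's aggroPercent to fill the bar, turning it red when full and hiding it at zero.
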(event EventBeginPlay
  ;[1 1 1] Set references
  (bind _outactors (Actor|GetAllActorsOfClass "/Game/Blueprints/StealthCharacter.StealthCharacter_C"))
  (bind _output_get (Variables|Default|SettargetPlayer (Utilities|Array|Get(acopy) _outactors)))
  (Variables|Default|SetplayerCamera (Variables|/Game/Blueprints/StealthCharacter.StealthCharacter_C|GetFollowCamera _output_get))
  (bind _asbp_aic_nullifier (Utilities|Casting|CastToBP_AIC_Nullifier (Pawn|GetController)))
  (Variables|Default|SetnullifierAIC _asbp_aic_nullifier)
  (bind _asbp_enemy_awareness (Utilities|Casting|CastToBP_EnemyAwareness (UserInterface|GetUserWidgetObject (Variables|Default|GetEnemyAwarenessIndicator))))
  (bind _output_get_2 (Variables|Default|SetawarenessWidget _asbp_enemy_awareness))
  (Variables|Default|SetawarenessBar (Variables|/Game/Blueprints/BP_EnemyAwareness.BP_EnemyAwareness_C|GetProgressBar_24 _output_get_2)))

(event Collision|EventActorBeginOverlap
  (params (OtherActor :type Actor%20Object%20Reference)))

(event EventTick
  (params (DeltaSeconds :type Float%20%28single-precision%29))
  (bind _returnvalue (Utilities|Name|MakeLiteralName "aggroPercent"))
  (bind _enemyawarenessindicator (Variables|Default|GetEnemyAwarenessIndicator))
  (bind _awarenesswidget (Variables|Default|GetawarenessWidget))
  (bind _awarenessbar (Variables|Default|GetawarenessBar))
  (bind _nullifieraic (Variables|Default|GetnullifierAIC))
  (bind _returnvalue_2 (AI|GetBlackboard _nullifieraic))
  (bind _returnvalue_3 (Class|BlackboardComponent|GetValueasFloat _returnvalue_2 _returnvalue))
  (bind _returnvalue_4 (Math|Float|Truncate _returnvalue_3))
  ;[1 1 1] Rotate indicator to face player camera
  (Transformation|SetWorldRotation _enemyawarenessindicator (Math|Rotator|MakeRotator 0.0 0.0 (.yaw (Math|Rotator|FindLookatRotation (Transformation|GetWorldLocation _enemyawarenessindicator) (Transformation|GetWorldLocation (Variables|Default|GetplayerCamera))))) false false)
  ;[1 1 1] Set awareness bar percent
  (Progress|SetPercent (Variables|Default|GetawarenessBar) (/ _returnvalue_3 1e+02))
  ;[1 1 1] Set fill colour
  (if (== _returnvalue_4 100)
    (Class|ProgressBar|SetFillColorandOpacity _awarenessbar "(R=1.000000,G=0.000000,B=0.000000,A=1.000000)")
    (else
      (Class|ProgressBar|SetFillColorandOpacity _awarenessbar "(R=0.750000,G=0.625000,B=0.000000,A=1.000000)")))
  ;[1 1 1] Set bar visibility
  (if (== _returnvalue_4 0)
    (Widget|SetVisibility _awarenesswidget "Hidden")
    (else
      (Widget|SetVisibility _awarenesswidget "Visible"))))

(fn ConstructionScript)