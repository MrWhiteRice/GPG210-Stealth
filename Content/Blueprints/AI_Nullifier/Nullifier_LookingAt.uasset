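; Behavior tree decorator for the Nullifier AI that tests its facing toward the stealth character stored in the targetToFollow blackboard key.
; It builds a rotator from the pawn's current roll and pitch plus the look-at yaw to the target, so only horizontal facing matters.
; Despite the LookingAt name, it passes when that rotator differs from the pawn's rotation beyond Lenience, meaning the Nullifier is not facing the target.
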(fn PerformConditionCheck
  (params (OwnerActor :type Actor%20Object%20Reference))
  ;[1 1 1] Get a reference to the controller
  (bind _asbp_aic_nullifier (Utilities|Casting|CastToBP_AIC_Nullifier OwnerActor))
  (bind _output_get (Variables|Default|SetnullifierAIC _asbp_aic_nullifier))
  ;[1 1 1] Determine if the AI is facing the target
  (bind _asstealth_character (Utilities|Casting|CastToStealthCharacter (AI|Components|Blackboard|GetValueasObject (AI|GetBlackboard _output_get) (Utilities|Name|MakeLiteralName "targetToFollow"))))
  (return (Utilities|Enum|NotEqual(Enum) (Math|Rotator|MakeRotator (.Roll (Math|Rotator|BreakRotator (.rotation (Transformation|GetActorTransform (Pawn|GetControlledPawn _output_get))))) (.Pitch (Math|Rotator|BreakRotator (.rotation (Transformation|GetActorTransform (Pawn|GetControlledPawn _output_get))))) (.yaw (Math|Rotator|FindLookatRotation (.location (Transformation|GetActorTransform (Pawn|GetControlledPawn _output_get))) (Transformation|GetActorLocation _asstealth_character)))) (.rotation (Transformation|GetActorTransform (Pawn|GetControlledPawn _output_get))) (Variables|Default|Getlenience))))