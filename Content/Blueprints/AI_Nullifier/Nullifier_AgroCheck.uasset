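; Behavior tree node for the Nullifier AI that detects targets for it to follow.
; Each tick it sphere-traces around the pawn for target object types, ignoring other Nullifiers, then line-traces to each hit on the Camera channel.
; A visible hit writes TargetToFollow and TargetLocation to the blackboard; a blocked one clears only TargetToFollow.
; Every hit is processed, so the last one decides the target.
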(event EventTick
  (params (OwnerActor :type Actor%20Object%20Reference) (DeltaSeconds :type Float%20%28single-precision%29))
  ;[1 1 1] Get a reference to the controller if there is none
  (if (!= (Variables|Default|GetnullifierAIC) 0)
    _
    (else
      (bind _asbp_aic_nullifier (Utilities|Casting|CastToBP_AIC_Nullifier OwnerActor))
      (Variables|Default|SetnullifierAIC _asbp_aic_nullifier)))
  ;[1 1 1] Get actors(enemies) to ignore
  (bind _outactors (Actor|GetAllActorsOfClass "/Game/Blueprints/AI_Nullifier/BP_AI_Nullifier.BP_AI_Nullifier_C"))
  ;[1 1 1] Set the current location of the AI
  (bind _output_get (Variables|Default|SetcurrentLocation (Transformation|GetActorLocation (Pawn|GetControlledPawn (Variables|Default|GetnullifierAIC)))))
  ;[1 1 1] Find players in range
  (bind _outhits (Collision|MultiSphereTraceForObjects _output_get (+ _output_get "0, 0,15.000000") 1.5e+03 (Variables|Default|GetdesiredTargetTypes) false _outactors "None"))
  ;[1 1 1] Determine if there is clear line of sight
  (bind _array_element (Utilities|Array|ForEachLoopwithBreak _outhits)
    (:LoopBody
      (bind _outhit (Collision|LineTraceByChannel (Variables|Default|GetcurrentLocation) (Transformation|GetActorLocation (.HitActor (Collision|BreakHitResult _array_element))) "TraceTypeQuery2" false _outactors "ForDuration"))
      ;[1 1 1] If there was line of sight, set values. Else, set values to null
      (if (== (.HitActor (Collision|BreakHitResult _outhit)) (.HitActor (Collision|BreakHitResult _array_element)))
        (Class|BTFunctionLibrary|SetBlackboardValueasObject (Variables|Default|GettargetToFollow) (.HitActor (Collision|BreakHitResult _outhit)))
        (AI|BehaviorTree|SetBlackboardValueasVector (Variables|Default|GettargetLocation) (Transformation|GetActorLocation (.HitActor (Collision|BreakHitResult _outhit))))
        (else
          (Class|BTFunctionLibrary|SetBlackboardValueasObject (Variables|Default|GettargetToFollow)))))))