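; BP_StormGrenade is a storm area-of-effect actor that destroys itself after a fixed lifespan.
; Tick widens StormArea horizontally along a sine ease-out curve up to MaxSize.
; Overlapping patrols, drones and nullifiers are recorded, but only nullifiers react, via CheckStormState, and are reset when the grenade is destroyed.
; Patrol and drone branches only print debug strings, and the cached player reference is never used.
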(event EventBeginPlay
  ;[1 1 1] Set lifespan
  (Actor|SetLifeSpan 1e+01)
  ;[1 1 1] Get reference to player
  (bind _outactors (Actor|GetAllActorsOfClass "/Game/Blueprints/StealthCharacter.StealthCharacter_C"))
  (Variables|Default|SetplayerToIgnore (Utilities|Array|Get(acopy) _outactors)))

(event Collision|EventActorBeginOverlap
  (params (OtherActor :type Actor%20Object%20Reference))
  ;[1 1 1] Is the character an enemy?
  (bind _ascharacter (Utilities|Casting|CastToCharacter OtherActor))
  (if (Utilities|Array|ContainsItem (Utilities|Array|MakeArray "/Game/Blueprints/AI_Patrol/BP_Patrol.BP_Patrol_C" "/Game/Blueprints/AI_Drone/BP_TempDrone.BP_TempDrone_C" "/Game/Blueprints/AI_Nullifier/BP_AI_Nullifier.BP_AI_Nullifier_C") (Utilities|GetClass _ascharacter))
    (Development|PrintString "test a")
    (Utilities|Array|Add (Variables|Default|GetaffectedCharacters) _ascharacter)
    (Utilities|Casting|CastToBP_Patrol _ascharacter
      (:then
        (Development|PrintString "patrol"))
      (:CastFailed
        (Development|PrintString "test b")
        (Utilities|Casting|CastToBP_TempDrone _ascharacter
          (:then
            (Development|PrintString "drone"))
          (:CastFailed
            (Development|PrintString "test c")
            (bind _asbp_ai_nullifier (Utilities|Casting|CastToBP_AI_Nullifier _ascharacter))
            (Development|PrintString "nullifier")
            (Default|CheckStormState _asbp_ai_nullifier self)))))))

(event EventTick
  (params (DeltaSeconds :type Float%20%28single-precision%29))
  (bind _storm_area_ (Variables|Default|GetStorm%20Area%20))
  ;[1 1 1] Expand over time
  (bind _output_get (Variables|Default|SetcurrentSize (+ (* DeltaSeconds 25.0) (Variables|Default|GetcurrentSize))))
  (Transformation|SetWorldScale3D _storm_area_ (Math|Vector|MakeVector (* (Math|Trig|Sin(Degrees) (Math|Float|Min(Float) _output_get 9e+01)) (Variables|Default|GetMaxSize)) (* (Math|Trig|Sin(Degrees) (Math|Float|Min(Float) _output_get 9e+01)) (Variables|Default|GetMaxSize)) (.z (Transformation|GetWorldScale _storm_area_)))))

(event EventDestroyed
  (for _array_element (Variables|Default|GetaffectedCharacters)
    (Utilities|Casting|CastToBP_Patrol _array_element
      (:CastFailed
        (Utilities|Casting|CastToBP_TempDrone _array_element
          (:CastFailed
            (bind _asbp_ai_nullifier (Utilities|Casting|CastToBP_AI_Nullifier _array_element))
            (Default|ResetStormState _asbp_ai_nullifier)))))))

(fn ConstructionScript)